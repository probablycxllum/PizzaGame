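; Temporary pizza pickup actor that lets the player take a pepperoni, cheese or sausage pizza from one of three trigger boxes.
; Box overlaps toggle per-box in-range flags, and BeginPlay binds the first-person character's interaction event to the pickup handler.
; The handler sets type flags for the first in-range box and prints it.
; The sausage branch clears its own flag and leaves cheese unchanged.
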(event `self.Box2.OnComponentBeginOverlap`
  (params (OverlappedComponent :type "PrimitiveComponent Object Reference") (OtherActor :type "Actor Object Reference") (OtherComp :type "PrimitiveComponent Object Reference") (OtherBodyIndex :type Integer) (bFromSweep :type Boolean) (SweepResult :type "HitResult Structure (by ref)"))
  ; box 1
  (set `self.inRange2` true))

(event `self.Box3.OnComponentBeginOverlap`
  (params (OverlappedComponent :type "PrimitiveComponent Object Reference") (OtherActor :type "Actor Object Reference") (OtherComp :type "PrimitiveComponent Object Reference") (OtherBodyIndex :type Integer) (bFromSweep :type Boolean) (SweepResult :type "HitResult Structure (by ref)"))
  ; box 2
  (set `self.inRange3` true))

(event `self.Box3.OnComponentEndOverlap`
  (params (OverlappedComponent :type "PrimitiveComponent Object Reference") (OtherActor :type "Actor Object Reference") (OtherComp :type "PrimitiveComponent Object Reference") (OtherBodyIndex :type Integer))
  ; box 2
  (set `self.inRange3` false))

(event `self.Box2.OnComponentEndOverlap`
  (params (OverlappedComponent :type "PrimitiveComponent Object Reference") (OtherActor :type "Actor Object Reference") (OtherComp :type "PrimitiveComponent Object Reference") (OtherBodyIndex :type Integer))
  ; box 1
  (set `self.inRange2` false))

(event `playerInteract`
  (if (`self.inRange1`)
    (set `self.hasPepperoni` true)
    (set `self.hasCheese` false)
    (set `self.hasSausage` false)
    (`KismetSystemLibrary.PrintString` "has peperoni")
    (elif (`self.inRange2`)
      (set `self.hasCheese` true)
      (set `self.hasPepperoni` false)
      (set `self.hasSausage` false)
      (`KismetSystemLibrary.PrintString` "has cheese")
      (elif (`self.inRange3`)
        (set `self.hasSausage` true)
        (set `self.hasPepperoni` false)
        (set `self.hasSausage` false)
        (`KismetSystemLibrary.PrintString` "has sausage")))))

(event `self.Box1.OnComponentBeginOverlap`
  (params (OverlappedComponent :type "PrimitiveComponent Object Reference") (OtherActor :type "Actor Object Reference") (OtherComp :type "PrimitiveComponent Object Reference") (OtherBodyIndex :type Integer) (bFromSweep :type Boolean) (SweepResult :type "HitResult Structure (by ref)"))
  ; box 3
  (set `self.inRange1` true))

(event `self.Box1.OnComponentEndOverlap`
  (params (OverlappedComponent :type "PrimitiveComponent Object Reference") (OtherActor :type "Actor Object Reference") (OtherComp :type "PrimitiveComponent Object Reference") (OtherBodyIndex :type Integer))
  ; box 3
  (set `self.inRange1` false))

(event `self.ReceiveBeginPlay`
  (bind _returnvalue (`GameplayStatics.GetActorOfClass` "/Game/FirstPerson/Blueprints/BP_FirstPersonCharacter.BP_FirstPersonCharacter_C"))
  (add `/Game/FirstPerson/Blueprints/BP_FirstPersonCharacter.OnInteraction` _returnvalue (delegate `playerInteract`)))

(fn `UserConstructionScript`)