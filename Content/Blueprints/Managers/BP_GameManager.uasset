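; BP_GameManager is a manager Blueprint that shows the day-over screen when an in-game day ends.
; On BeginPlay it creates the WBP_DayOver widget up front, finds the level's BP_DayManager and binds to its DayOverDispatcher.
; When that dispatcher fires, it adds the stored widget to the viewport and switches player 0 to UI-only input focused on the widget.
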(event `self.ReceiveBeginPlay`
  (`self.CreateWidgets`)
  (bind _returnvalue (`GameplayStatics.GetActorOfClass` "/Game/Blueprints/Managers/BP_DayManager.BP_DayManager_C"))
  (bind _output_get (set `self.BP_DayManager` _returnvalue))
  (add `/Game/Blueprints/Managers/BP_DayManager.DayOverDispatcher` _output_get (delegate `DayOverHandler`)))

(event `DayOverHandler`
  (`UserWidget.AddToViewport` (`self.WBP_DayOverWidget`) 0)
  (`WidgetBlueprintLibrary.SetInputMode_UIOnlyEx` (`GameplayStatics.GetPlayerController` 0) (`self.WBP_DayOverWidget`)))

(fn `CreateWidgets`
  (locals (NewLocalVar :type "/Game/Blueprints/UI/WBP_DayOver Object Reference"))
  (bind _returnvalue (`|CreateWidget` "/Game/Blueprints/UI/WBP_DayOver.WBP_DayOver_C"))
  (set `self.WBP_DayOverWidget` _returnvalue))

(fn `UserConstructionScript`)