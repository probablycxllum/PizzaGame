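; BP_DayManager is a manager Blueprint that tracks the game's current hour and day.
; A looping one-second timer started on BeginPlay counts down the remaining time and advances the hour every 25 ticks.
; UpdateTimer runs each tick and increments the day whenever the countdown is at or below zero, with no reset of countdown or hour shown.
; CallUpdateCurrentHourUI is called only at BeginPlay.
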(event `self.ReceiveBeginPlay`
  (bind _returnvalue (`KismetSystemLibrary.K2_SetTimerDelegate` (delegate `UpdateDayTime`) 1.0 true))
  (set `self.DayTimerHandle` _returnvalue)
  (`self.UpdateCurrentHourUI`))

(event `UpdateDayTime`
  (set `self.F_HourCounter` (+ (`self.F_HourCounter`) 1))
  (set `self.F_CurrentTime` (- (`self.F_CurrentTime`) 1.0))
  (if (>= (`self.F_HourCounter`) 25)
    (set `self.F_HourCounter` 0)
    (set `self.I_CurrentHour` (+ (`self.I_CurrentHour`) 1))
    (`self.UpdateTimer`)
    (else
      (`self.UpdateTimer`))))

(fn `UpdateTimer`
  (if (<= (`self.F_CurrentTime`) 0.0)
    (set `self.I_CurrentDay` (+ (`self.I_CurrentDay`) 1))))

(fn `UserConstructionScript`)