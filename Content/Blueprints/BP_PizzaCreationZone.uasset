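; BP_PizzaCreationZone is an interaction zone that switches the player into a pizza build mode.
; On BeginPlay it binds EnterBuildMode to the first-person character's OnInteraction dispatcher, gated by a flag that box overlap sets and clears without filtering actors.
; Entering build mode blends the view to the zone actor, ignores move and look input and shows the mouse cursor, with no exit logic in this Blueprint.
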(event `self.ReceiveBeginPlay`
  (bind _returnvalue (`GameplayStatics.GetActorOfClass` "/Game/FirstPerson/Blueprints/BP_FirstPersonCharacter.BP_FirstPersonCharacter_C"))
  (add `/Game/FirstPerson/Blueprints/BP_FirstPersonCharacter.OnInteraction` _returnvalue (delegate `EnterBuildMode`)))

(event `EnterBuildMode`
  (bind _returnvalue (`GameplayStatics.GetPlayerController` 0))
  (if (`self.B_CanInteract`)
    (`PlayerController.SetViewTargetWithBlend` _returnvalue self 1.0 "VTBlend_Linear" 0.0 false)
    (`Controller.SetIgnoreMoveInput` _returnvalue true)
    (`Controller.SetIgnoreLookInput` _returnvalue true)
    (set `PlayerController.bShowMouseCursor` true _returnvalue)))

(event `self.Box.OnComponentBeginOverlap`
  (params (OverlappedComponent :type "PrimitiveComponent Object Reference") (OtherActor :type "Actor Object Reference") (OtherComp :type "PrimitiveComponent Object Reference") (OtherBodyIndex :type Integer) (bFromSweep :type Boolean) (SweepResult :type "HitResult Structure (by ref)"))
  (set `self.B_CanInteract` true))

(event `self.Box.OnComponentEndOverlap`
  (params (OverlappedComponent :type "PrimitiveComponent Object Reference") (OtherActor :type "Actor Object Reference") (OtherComp :type "PrimitiveComponent Object Reference") (OtherBodyIndex :type Integer))
  (set `self.B_CanInteract` false))

(fn `UserConstructionScript`)